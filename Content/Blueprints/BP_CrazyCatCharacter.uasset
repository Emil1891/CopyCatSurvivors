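; Player character Blueprint for CopyCat Survivors, handling sprite feedback, a survival timer, level-ups and death.
; Tick plays footsteps on a flipbook frame, mirrors the sprite by Y velocity and counts minutes/seconds through a Delay.
; XP gains raise the pickup sound's pitch with progress, while level-ups shuffle CatManager's cats and offer up to three in a paused menu.
; Death swaps to a death flipbook, then hides the sprite and pauses on the game-over widget.
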(event Collision|EventActorBeginOverlap
  (params (OtherActor :type Actor%20Object%20Reference)))

(event EventTick
  (params (DeltaSeconds :type Float%20%28single-precision%29))
  (bind _paperflipbook (Variables|Default|GetPaperFlipbook))
  (Utilities|FlowControl|Sequence
    (:then_1
      ;[1 1 1] Plays footstep sound
      (if (and (> (Math|Vector|VectorLength (Variables|/Script/Engine.MovementComponent|GetVelocity (Pawn|GetMovementComponent))) 0.1) (== (Class|PaperFlipbookComponent|GetPlaybackPositioninFrames (Variables|Default|GetPaperFlipbook)) 2))
        (Audio|PlaySound2D "/Game/Audio/mc_footsteps.mc_footsteps" 1.0 1.0 0.0 0 0)))
    (:then_2
      ;[1 1 1] Flips character in movement direction
      (Math|Float|CompareFloat (.Y (Class|KismetMathLibrary|BreakVector3f (Variables|/Script/Engine.MovementComponent|GetVelocity (Pawn|GetMovementComponent)))) 0.0
        (:>
          (Transformation|SetRelativeScale3D _paperflipbook "-4.000000,4.000000,4.000000"))
        (:<
          (Transformation|SetRelativeScale3D _paperflipbook "4.000000,4.000000,4.000000"))))
    (:then_3
      (Utilities|FlowControl|Delay 1.0)
      (Variables|Default|SetSeconds (+ (Variables|Default|GetSeconds) 1))
      (if (> (Variables|Default|GetSeconds) 59)
        (Variables|Default|SetMinutes (+ (Variables|Default|GetMinutes) 1))
        (Variables|Default|SetSeconds 0)))))

(event EventLevelUpEvent
  (bind _returnvalue (Game|GetPlayerController 0))
  (Audio|PlaySound2D "/Game/Audio/Jump_014.Jump_014" 1.0 1.0 0.0 0 0)
  (Utilities|IsValid (Variables|Default|GetSelectCatMenu)
    (:Is%20Valid
      _)
    (:Is%20Not%20Valid
      (bind _returnvalue_2 (UserInterface|CreateWidget "/Game/UI/UBWP_ChooseCatMenu.UBWP_ChooseCatMenu_C"))
      (bind _output_get (Variables|Default|SetSelectCatMenu _returnvalue_2))
      (Variables|/Game/UI/UBWP_ChooseCatMenu.UBWP_ChooseCatMenu_C|SetCatManager _output_get (Variables|Default|GetCatManager))))
  (Variables|/Script/Engine.PlayerController|SetbShowMouseCursor _returnvalue true)
  (bind _ascopy_cat_survivors_player_controller (Utilities|Casting|CastToCopyCatSurvivorsPlayerController _returnvalue)
    (:then
      (Variables|/Script/CopyCatSurvivors.CopyCatSurvivorsPlayerController|SetbDoLaser _ascopy_cat_survivors_player_controller false))
    (:CastFailed
      _))
  (Utilities|Array|Shuffle (Variables|/Script/CopyCatSurvivors.CatManager|GetCats (Variables|Default|GetCatManager)))
  (Utilities|FlowControl|Sequence
    (:then_0
      (if (>= (Utilities|Array|Length (Variables|/Script/CopyCatSurvivors.CatManager|GetCats (Variables|Default|GetCatManager))) 1)
        (Variables|/Game/UI/UBWP_ChooseCatMenu.UBWP_ChooseCatMenu_C|SetCat1Ref (Variables|Default|GetSelectCatMenu) (Utilities|Array|Get(acopy) (Variables|/Script/CopyCatSurvivors.CatManager|GetCats (Variables|Default|GetCatManager))))))
    (:then_1
      (if (>= (Utilities|Array|Length (Variables|/Script/CopyCatSurvivors.CatManager|GetCats (Variables|Default|GetCatManager))) 2)
        (Variables|/Game/UI/UBWP_ChooseCatMenu.UBWP_ChooseCatMenu_C|SetCat2Ref (Variables|Default|GetSelectCatMenu) (Utilities|Array|Get(acopy) (Variables|/Script/CopyCatSurvivors.CatManager|GetCats (Variables|Default|GetCatManager)) 1))))
    (:then_2
      (if (>= (Utilities|Array|Length (Variables|/Script/CopyCatSurvivors.CatManager|GetCats (Variables|Default|GetCatManager))) 3)
        (Variables|/Game/UI/UBWP_ChooseCatMenu.UBWP_ChooseCatMenu_C|SetCat3Ref (Variables|Default|GetSelectCatMenu) (Utilities|Array|Get(acopy) (Variables|/Script/CopyCatSurvivors.CatManager|GetCats (Variables|Default|GetCatManager)) 2))))
    (:then_3
      (Input|SetInputModeUIOnly _returnvalue (Variables|Default|GetSelectCatMenu) "DoNotLock" false)
      (UserInterface|Viewport|AddtoViewport (Variables|Default|GetSelectCatMenu) 0)
      (Game|SetGamePaused true)
      (Variables|/Script/Engine.PlayerController|SetbShowMouseCursor (Game|GetPlayerController 0) true))))

(event EventOnKillMeEvent
  (bind _returnvalue (Game|GetPlayerController 0))
  (Sprite|SetFlipbook (Variables|Default|GetPaperFlipbook) "/Game/2D/MainCharacter/FB_MainChar_Death.FB_MainChar_Death")
  (Utilities|FlowControl|Delay 1.0)
  (Development|SetHiddeninGame (Variables|Default|GetPaperFlipbook) true false)
  (Utilities|IsValid (Variables|Default|GetGameOverWidget)
    (:Is%20Valid
      _)
    (:Is%20Not%20Valid
      (bind _returnvalue_2 (UserInterface|CreateWidget "/Game/UI/UBWP_GameOver.UBWP_GameOver_C"))
      (Variables|Default|SetGameOverWidget _returnvalue_2)))
  (bind _ascopy_cat_survivors_player_controller (Utilities|Casting|CastToCopyCatSurvivorsPlayerController _returnvalue)
    (:then
      (Variables|/Script/CopyCatSurvivors.CopyCatSurvivorsPlayerController|SetbDoLaser _ascopy_cat_survivors_player_controller false)
      (Input|SetInputModeUIOnly _returnvalue (Variables|Default|GetGameOverWidget) "DoNotLock" false)
      (UserInterface|Viewport|AddtoViewport (Variables|Default|GetGameOverWidget) 0)
      (Game|SetGamePaused true))
    (:CastFailed
      (Development|PrintString "NoController"))))

(event EventOnIncreasedXP
  (bind _gem_pickup2 (Variables|Default|Getgem_pickup2))
  ;[1 1 1] Dynamic pitch on pickup sound
  (Audio|Components|Audio|SetPitchMultiplier _gem_pickup2 (+ 1.0 (/ (Class|CrazyCatCharacter|GetXPPercent) 1.5)))
  (Audio|Components|Audio|Play _gem_pickup2 0.0))

(fn ConstructionScript)