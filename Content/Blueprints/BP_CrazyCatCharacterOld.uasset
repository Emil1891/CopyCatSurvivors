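; BP_CrazyCatCharacterOld is a cat game character with a Paper2D flipbook and a level-up cat selection menu.
; Tick mirrors the flipbook by flipping its X scale according to the sign of Y velocity.
; LevelUpEvent lazily creates the choose-cat widget, shuffles the CatManager's cats and passes up to three to it.
; It then shows the cursor and menu, switches to UI-only input and pauses the game.
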(event EventBeginPlay)

(event Collision|EventActorBeginOverlap
  (params (OtherActor :type Actor%20Object%20Reference)))

(event EventTick
  (params (DeltaSeconds :type Float%20%28single-precision%29))
  (bind _paperflipbook (Variables|Default|GetPaperFlipbook))
  (Math|Float|CompareFloat (.Y (Class|KismetMathLibrary|BreakVector3f (Variables|/Script/Engine.MovementComponent|GetVelocity (Pawn|GetMovementComponent)))) 0.0
    (:>
      (Transformation|SetRelativeScale3D _paperflipbook "-4.000000,4.000000,4.000000"))
    (:<
      (Transformation|SetRelativeScale3D _paperflipbook "4.000000,4.000000,4.000000"))))

(event EventLevelUpEvent
  (bind _returnvalue (Game|GetPlayerController 0))
  (Utilities|IsValid (Variables|Default|GetSelectCatMenu)
    (:Is%20Valid
      _)
    (:Is%20Not%20Valid
      (bind _returnvalue_2 (UserInterface|CreateWidget "/Game/UI/UBWP_ChooseCatMenu.UBWP_ChooseCatMenu_C"))
      (bind _output_get (Variables|Default|SetSelectCatMenu _returnvalue_2))
      (Variables|/Game/UI/UBWP_ChooseCatMenu.UBWP_ChooseCatMenu_C|SetCatManager _output_get (Variables|Default|GetCatManager))))
  (Variables|/Script/Engine.PlayerController|SetbShowMouseCursor _returnvalue true)
  (Utilities|Array|Shuffle (Variables|/Script/CopyCatSurvivors.CatManager|GetCats (Variables|Default|GetCatManager)))
  (Utilities|FlowControl|Sequence
    (:then_0
      (if (>= (Utilities|Array|Length (Variables|/Script/CopyCatSurvivors.CatManager|GetCats (Variables|Default|GetCatManager))) 1)
        (Variables|/Game/UI/UBWP_ChooseCatMenu.UBWP_ChooseCatMenu_C|SetCat1Ref (Variables|Default|GetSelectCatMenu) (Utilities|Array|Get(acopy) (Variables|/Script/CopyCatSurvivors.CatManager|GetCats (Variables|Default|GetCatManager))))))
    (:then_1
      (if (>= (Utilities|Array|Length (Variables|/Script/CopyCatSurvivors.CatManager|GetCats (Variables|Default|GetCatManager))) 2)
        (Variables|/Game/UI/UBWP_ChooseCatMenu.UBWP_ChooseCatMenu_C|SetCat2Ref (Variables|Default|GetSelectCatMenu) (Utilities|Array|Get(acopy) (Variables|/Script/CopyCatSurvivors.CatManager|GetCats (Variables|Default|GetCatManager)) 1))))
    (:then_2
      (if (>= (Utilities|Array|Length (Variables|/Script/CopyCatSurvivors.CatManager|GetCats (Variables|Default|GetCatManager))) 3)
        (Variables|/Game/UI/UBWP_ChooseCatMenu.UBWP_ChooseCatMenu_C|SetCat3Ref (Variables|Default|GetSelectCatMenu) (Utilities|Array|Get(acopy) (Variables|/Script/CopyCatSurvivors.CatManager|GetCats (Variables|Default|GetCatManager)) 2))))
    (:then_3
      (Input|SetInputModeUIOnly _returnvalue (Variables|Default|GetSelectCatMenu) "DoNotLock" false)
      (UserInterface|Viewport|AddtoViewport (Variables|Default|GetSelectCatMenu) 0)
      (Game|SetGamePaused true))))

(fn ConstructionScript)